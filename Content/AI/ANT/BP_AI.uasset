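; Enemy ant AI character that spots the player, melee attacks and dies from damage.
; Pawn sensing sets a blackboard flag when it sees the player.
; AttackPlayer sphere-traces forward, then plays an attack montage and applies damage to a player hit.
; Damage halts movement and plays random reactions; at zero health it plays a death montage, destroys itself and decrements the game mode's alive count.
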(event OnSeePawn(PawnSensing)
  (params (Pawn :type Pawn%20Object%20Reference))
  (Utilities|Casting|CastToBP_FirstPersonCharacter Pawn)
  (AI|Components|Blackboard|SetValueasBool (AI|GetBlackboard (AI|GetAIController self)) (Utilities|Name|MakeLiteralName "HasSeenPlayer?") true))

(event Custom|Attack%20Player
  (bind _returnvalue (Transformation|GetActorLocation))
  (bind (_outhit _returnvalue_2) (Collision|SphereTraceForObjects _returnvalue (+ _returnvalue (* (Math|Vector|GetForwardVector (Transformation|GetActorRotation)) 2.5e+02)) 9e+01 (Utilities|Array|MakeArray "ObjectTypeQuery3") false 0 "None"))
  (if _returnvalue_2
    (Utilities|Casting|CastToBP_FirstPersonCharacter (.HitActor (Collision|BreakHitResult _outhit)))
    (Animation|PlayAnimMontage "/Game/AI/Animations/Ant/AS_Ant_Attack2_Montage2.AS_Ant_Attack2_Montage2" 1.0 "None")
    (Game|Damage|ApplyDamage (.HitActor (Collision|BreakHitResult _outhit)) 1e+01 0 0)))

(event EventBeginPlay
  (bind _asbp_first_person_game_mode (Utilities|Casting|CastToBP_FirstPersonGameMode (Game|GetGameMode)))
  (Variables|/Game/FirstPerson/Blueprints/BP_FirstPersonGameMode.BP_FirstPersonGameMode_C|SetAmount%20Alive _asbp_first_person_game_mode (- (Variables|/Game/FirstPerson/Blueprints/BP_FirstPersonGameMode.BP_FirstPersonGameMode_C|GetAmount%20Alive _asbp_first_person_game_mode) 0)))

(event Collision|EventActorBeginOverlap
  (params (OtherActor :type Actor%20Object%20Reference)))

(event EventTick
  (params (DeltaSeconds :type Float%20%28single-precision%29)))

(event Game|Damage|EventAnyDamage
  (params (Damage :type Float%20%28single-precision%29) (DamageType :type Damage%20Type%20Object%20Reference) (InstigatedBy :type Controller%20Object%20Reference) (DamageCauser :type Actor%20Object%20Reference))
  (bind _charactermovement (Variables|Character|GetCharacterMovement))
  (Components|Movement|StopMovementImmediately (Variables|Character|GetCharacterMovement))
  (Animation|PlayAnimMontage (Utilities|Select :Index (Math|Random|RandomIntegerinRange 0 3) :Option%200 "/Game/Characters/Insects/Ant/Animation/AS_Ant_Taking_Damage_V1_R_Montage.AS_Ant_Taking_Damage_V1_R_Montage" :Option%201 "/Game/Characters/Insects/Ant/Animation/AS_Ant_Taking_Damage_V1_L_Montage.AS_Ant_Taking_Damage_V1_L_Montage" :Option%202 "/Game/Characters/Insects/Ant/Animation/AS_Ant_Taking_Damage_V2_L_Montage.AS_Ant_Taking_Damage_V2_L_Montage" :Option%203 "/Game/Characters/Insects/Ant/Animation/AS_Ant_Taking_Damage_V2_R_Montage.AS_Ant_Taking_Damage_V2_R_Montage") 0.9 "None")
  (Variables|Default|SetHealth (- (Variables|Default|GetHealth) Damage))
  (if (<= (Variables|Default|GetHealth) 0.0)
    (Variables|Default|SetisDead? true)
    (Class|NavMovementComponent|StopActiveMovement _charactermovement)
    (Components|Movement|StopMovementImmediately _charactermovement)
    (bind _returnvalue (Animation|PlayAnimMontage (Utilities|Select :Index (Math|Random|RandomIntegerinRange 0 1) :Option%200 "/Game/Characters/Insects/Ant/Animation/AS_Ant_Death_V2_Montage.AS_Ant_Death_V2_Montage" :Option%201 "/Game/Characters/Insects/Ant/Animation/AS_Ant_Death_V1_Montage.AS_Ant_Death_V1_Montage" :Option%202 0) 0.7 "None"))
    (Utilities|FlowControl|Delay _returnvalue)
    (Actor|DestroyActor)
    (bind _asbp_first_person_game_mode (Utilities|Casting|CastToBP_FirstPersonGameMode (Game|GetGameMode)))
    (Variables|/Game/FirstPerson/Blueprints/BP_FirstPersonGameMode.BP_FirstPersonGameMode_C|SetAmount%20Alive _asbp_first_person_game_mode (Utilities|Operators|Subtract (Variables|/Game/FirstPerson/Blueprints/BP_FirstPersonGameMode.BP_FirstPersonGameMode_C|GetAmount%20Alive _asbp_first_person_game_mode) 1))))

(fn ConstructionScript)